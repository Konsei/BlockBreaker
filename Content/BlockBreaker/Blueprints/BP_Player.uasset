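; BP_Player is the player pawn for BlockBreaker, handling movement, look and the starting weapon.
; On BeginPlay it spawns a BP_Rifle, stores it as EquippedGun and snaps it to the GunLocation component.
; Axis inputs feed movement along the actor's forward and right vectors, and controller yaw and pitch for looking.
; It contains no firing logic, and Tick and overlap events are unused.
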(event EventBeginPlay
  (bind _returnvalue (Game|SpawnActorfromClass "/Game/BlockBreaker/Blueprints/BP_Rifle.BP_Rifle_C" (Math|Transform|MakeTransform "0, 0, 0" "0, 0, 0" "1,1,1") "Undefined" 0 0))
  (bind _output_get (Variables|Default|SetEquippedGun _returnvalue))
  (Transformation|AttachComponentToComponent _output_get (Variables|Default|GetGunLocation) "None" "SnapToTarget" "SnapToTarget" "KeepRelative" true))

(event Collision|EventActorBeginOverlap
  (params (OtherActor :type Actor%20Object%20Reference)))

(event EventTick
  (params (DeltaSeconds :type Float%20%28single-precision%29)))

(event Input|AxisEvents|InputAxisMoveForward
  (params (AxisValue :type Float%20%28single-precision%29))
  (Pawn|Input|AddMovementInput (Transformation|GetActorForwardVector) AxisValue false))

(event Input|AxisEvents|InputAxisMoveRight
  (params (AxisValue :type Float%20%28single-precision%29))
  (Pawn|Input|AddMovementInput (Transformation|GetActorRightVector) AxisValue false))

(event Input|AxisEvents|InputAxisLookHorizontal
  (params (AxisValue :type Float%20%28single-precision%29))
  (Pawn|Input|AddControllerYawInput AxisValue))

(event Input|AxisEvents|InputAxisLookVertical
  (params (AxisValue :type Float%20%28single-precision%29))
  (Pawn|Input|AddControllerPitchInput AxisValue))

(fn ConstructionScript)